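; Beach button actor that sinks when overlapped and spawns turtles of a configurable movement type.
; Collision overlap plays a sound and a timeline that lerps the button down, reversing it on exit.
; Timeline updates spawn a turtle at an offset from the button whenever the Tick-accumulated cooldown exceeds SpawnDelay.
; Tick also destroys tracked turtles overlapping Finish, without removing them from the array.
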(event `self.ReceiveBeginPlay`)

(event `self.ReceiveActorBeginOverlap`
  (params (OtherActor :type "Actor Object Reference"))
  (bind (_returnvalue_location _returnvalue_rotation _returnvalue_scale) (`KismetMathLibrary.BreakTransform` (`SceneComponent.GetRelativeTransform` (`self.Button`))))
  ;[1 1 1] Animation bounding positions
  (set `self.Out Position` (`KismetMathLibrary.MakeTransform` _returnvalue_location _returnvalue_rotation _returnvalue_scale))
  (set `self.In Position` (`KismetMathLibrary.MakeTransform` (- _returnvalue_location (0.0 0.0 10.0)) _returnvalue_rotation _returnvalue_scale)))

(event `self.Collision.OnComponentBeginOverlap`
  (params (OverlappedComponent :type "PrimitiveComponent Object Reference") (OtherActor :type "Actor Object Reference") (OtherComp :type "PrimitiveComponent Object Reference") (OtherBodyIndex :type Integer) (bFromSweep :type Boolean) (SweepResult :type "HitResult Structure (by ref)"))
  ;[1 1 1] Pressing animation
  (`GameplayStatics.PlaySoundAtLocation` "/Game/beach/sounds/Button_Sound.Button_Sound" (0.0 0.0 0.0) (struct) 1.0 1.0 0.0 null null null)
  (bind (_direction _newtrack_0) (`Timeline|ButtonTimelineIn` :!label _label)
    (:`Update`
      (`SceneComponent.K2_SetRelativeTransform` (`self.Button`) (`KismetMathLibrary.TLerp` (`self.Out Position`) (`self.In Position`) _newtrack_0) false false)
      ;[1 1 1] Spawn turtle
      (`/Engine/EditorBlueprintResources/StandardMacros.CompareFloat` (`self.spawn_delay`) (`self.last_spaw`)
        (:`<`
          (set `self.last_spaw` 0.0)
          (bind _returnvalue (`|SpawnActorFromClass` "/Game/beach/turtle/Turtle_Actor.Turtle_Actor_C" (`KismetMathLibrary.MakeTransform` (+ (`self.K2_GetActorLocation`) (+ (`self.GetActorForwardVector`) (500.0 0.0 200.0)))) "Undefined" "OverrideRootScale" null (`self.turtle_type`) null))
          (`KismetArrayLibrary.Array_Add` (`self.turtles`) _returnvalue))))))

(event `self.Collision.OnComponentEndOverlap`
  (params (OverlappedComponent :type "PrimitiveComponent Object Reference") (OtherActor :type "Actor Object Reference") (OtherComp :type "PrimitiveComponent Object Reference") (OtherBodyIndex :type Integer))
  (goto _label :!via `Reverse`))

(event `self.ReceiveTick`
  (params (DeltaSeconds :type "Float (single-precision)"))
  ;[1 1 1] Update variables
  (set `self.last_spaw` (+ DeltaSeconds (`self.last_spaw`)))
  ;[1 1 1] Remove turtle at finish
  (for _array_element (`self.turtles`)
    (if (`self.IsOverlappingActor` (`self.finish`) _array_element)
      (`self.K2_DestroyActor` _array_element))))

(fn `UserConstructionScript`)